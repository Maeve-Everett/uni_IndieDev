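; Enemy character that chases the player when pawn sensing spots a pawn and awards experience to the player when killed.
; Tick deals melee damage on a cooldown while the player is within close range.
; AnyDamage lowers health and destroys the enemy at zero.
; An overlay widget receives a reference to the enemy and rotates each frame to face the player camera.
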(event `self.ReceiveBeginPlay`
  (set `self.Health` (`self.MaxHealth`))
  (bind _aswbp_enemy_overlay (cast `/Game/UI/WBP_EnemyOverlay` (`WidgetComponent.GetWidget` (`self.HUDOverlay`))))
  (set `/Game/UI/WBP_EnemyOverlay.Enemy` self _aswbp_enemy_overlay))

(event `self.ReceiveAnyDamage`
  (params (Damage :type "Float (single-precision)") (DamageType :type "DamageType Object Reference") (InstigatedBy :type "Controller Object Reference") (DamageCauser :type "Actor Object Reference"))
  (bind _output_get (set `self.Health` (- (`self.Health`) Damage)))
  (if (<= _output_get 0.0)
    (bind _asbp_third_person_character (cast `/Game/ThirdPerson/Blueprints/BP_ThirdPersonCharacter` (`GameplayStatics.GetPlayerCharacter` 0)))
    (`/Game/ThirdPerson/Blueprints/BP_ThirdPersonCharacter.Gain Exp` _asbp_third_person_character (`self.ExpAwarded`))
    (`self.K2_DestroyActor`)))

(event `self.PawnSensing.OnSeePawn`
  (params (Pawn :type "Pawn Object Reference"))
  (`|AIMoveTo` self (0.0 0.0 0.0) (`GameplayStatics.GetPlayerPawn` 0)))

(event `self.ReceiveTick`
  (params (DeltaSeconds :type "Float (single-precision)"))
  (bind _hudoverlay (`self.HUDOverlay`))
  (`SceneComponent.K2_SetWorldRotation` _hudoverlay (`KismetMathLibrary.FindLookAtRotation` (`SceneComponent.K2_GetComponentLocation` _hudoverlay) (`PlayerCameraManager.GetCameraLocation` (`GameplayStatics.GetPlayerCameraManager` 0))) false false)
  (if (<= (`KismetMathLibrary.Vector_Distance` (`self.K2_GetActorLocation`) (`self.K2_GetActorLocation` (`GameplayStatics.GetPlayerPawn` 0))) 100.0)
    (bind _output_get (set `self.AttackCD` (- (`self.AttackCD`) DeltaSeconds)))
    (if (<= _output_get 0.0)
      (bind _asbp_third_person_character (cast `/Game/ThirdPerson/Blueprints/BP_ThirdPersonCharacter` (`GameplayStatics.GetPlayerPawn` 0)))
      (`/Game/ThirdPerson/Blueprints/BP_ThirdPersonCharacter.TakeDamage` _asbp_third_person_character 15.0)
      (set `self.AttackCD` 1.0))))

(fn `UserConstructionScript`)